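; Camera trigger volume that requests a camera change when the player character enters or leaves it.
; Overlap calls ChangeCamera with its Camera on entry and with no camera on exit, printing a debug message each time.
; Every Tick, regardless of overlap, the Camera turns toward the player and interpolates to the Spline point closest to them, forming a rail-style follow camera.
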(event EventBeginPlay)

(event Collision|EventActorEndOverlap
  (params (OtherActor :type Actor%20Object%20Reference))
  (if (== OtherActor (Game|GetPlayerCharacter 0))
    (Development|PrintString "PLAYER IS OUT")
    (Default|CallChangeCamera)))

(event Collision|EventActorBeginOverlap
  (params (OtherActor :type Actor%20Object%20Reference))
  (if (== OtherActor (Game|GetPlayerCharacter 0))
    (Development|PrintString "PLAYER IS IN")
    (Default|CallChangeCamera (Variables|Default|GetCamera))))

(event EventTick
  (params (DeltaSeconds :type Float%20%28single-precision%29))
  (bind _camera (Variables|Default|GetCamera))
  (bind _returnvalue (Transformation|GetActorLocation _camera))
  (Transformation|SetActorRotation (Variables|Default|GetCamera) (Math|Rotator|MakeRotationfromAxes (- (Transformation|GetActorLocation (Game|GetPlayerCharacter 0)) _returnvalue) "0, 0, 0" "0, 0, 0"))
  (Transformation|SetActorLocation (Variables|Default|GetCamera) (Math|Interpolation|VInterpTo _returnvalue (Spline|FindLocationClosesttoWorldLocation (Variables|Default|GetSpline) (Transformation|GetActorLocation (Game|GetPlayerCharacter 0)) "World") (Utilities|Time|GetWorldDeltaSeconds) 2e+01) false false))

(fn ConstructionScript)